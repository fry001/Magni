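; Slime enemy for a 2D-style Paper2D game that leaps at the nearby player, damages it on contact and dies at zero HP.
; Tick restarts a cooldown when the player is near and, on that frame, launches the sphere toward the player along X if within closer range.
; Velocity flips the sprite and picks stand or jump flipbooks, overridden by death.
; Hits damage \"player\"-tagged actors; lethal damage destroys the slime after a short delay.
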(event EventBeginPlay)

(event Collision|EventActorBeginOverlap
  (params (OtherActor :type Actor%20Object%20Reference)))

(event EventTick
  (params (DeltaSeconds :type Float%20%28single-precision%29))
  (bind _returnvalue (Game|Player|GetPlayerPawn 0))
  (bind _returnvalue_2 (Transformation|GetVelocity))
  ;[1 1 1] Настройки поведения и анимации слайма
  (Variables|Default|Setdt DeltaSeconds)
  (Variables|Default|Setpd (Transformation|GetDistanceTo _returnvalue))
  (Utilities|FlowControl|Sequence
    (:then_0
      (if (<= (Variables|Default|Getreset_tm) 0.0)
        (if (<= (Variables|Default|Getpd) 4e+02)
          (Variables|Default|Setreset_tm (Variables|Default|Getreset)))
        (else
          (Variables|Default|Setreset_tm (- (Variables|Default|Getreset_tm) (Variables|Default|Getdt))))))
    (:then_1
      (if (and (<= (Variables|Default|Getpd) 3e+02) (== (Variables|Default|Getreset_tm) (Variables|Default|Getreset)))
        (if (> (.X (Math|Vector|BreakVector (Transformation|GetActorLocation _returnvalue))) (.X (Math|Vector|BreakVector (Transformation|GetActorLocation))))
          (Variables|Default|SetXk 1.0)
          (else
            (Variables|Default|SetXk -1.0)))
        (Physics|AddImpulse (Variables|Default|GetSphere) (Math|Vector|MakeVector (* (Variables|Default|Getspd_x) (Variables|Default|GetXk)) 0.0 (Variables|Default|Getspd_z)) "None" true)))
    (:then_2
      (Utilities|FlowControl|Sequence
        (:then_0
          (if (> (.X (Math|Vector|BreakVector _returnvalue_2)) 0.0)
            (Transformation|SetWorldRotation (Variables|Default|GetPaperFlipbook) "0,180.000000, 0" false false)
            (else
              (Transformation|SetWorldRotation (Variables|Default|GetPaperFlipbook) "0,0.000000, 0" false false))))
        (:then_1
          (if (> (Math|Vector|VectorLength _returnvalue_2) 0.0)
            (Variables|Default|Setfb "/Game/2DSideScrollerBP/Sprites/slug01_jump.slug01_jump")
            (else
              (Variables|Default|Setfb "/Game/2DSideScrollerBP/Sprites/slug01_stand.slug01_stand"))))
        (:then_2
          (if (<= (Variables|Default|Gethp) 0.0)
            (Variables|Default|Setfb "/Game/2DSideScrollerBP/Sprites/slug01_death.slug01_death")))
        (:then_3
          (Sprite|SetFlipbook (Variables|Default|GetPaperFlipbook) (Variables|Default|Getfb)))))))

(event Collision|EventHit
  (params (MyComp :type Primitive%20Component%20Object%20Reference) (Other :type Actor%20Object%20Reference) (OtherComp :type Primitive%20Component%20Object%20Reference) (bSelfMoved :type Boolean) (HitLocation :type Vector :default "0, 0, 0") (HitNormal :type Vector :default "0, 0, 0") (NormalImpulse :type Vector :default "0, 0, 0") (Hit :type Hit%20Result%20Structure%20%28by%20ref%29))
  ;[1 1 1] Нанесеие урона актору с тэгом
  (if (Actor|ActorHasTag Other "player")
    (Game|Damage|ApplyDamage Other (Variables|Default|Getdmg_slime) 0 0)))

(event Game|Damage|EventAnyDamage
  (params (Damage :type Float%20%28single-precision%29) (DamageType :type Damage%20Type%20Object%20Reference) (InstigatedBy :type Controller%20Object%20Reference) (DamageCauser :type Actor%20Object%20Reference))
  ;[1 1 1] Получеие урона и смерть
  (bind _output_get (Variables|Default|Sethp (- (Variables|Default|Gethp) Damage)))
  (if (<= _output_get 0.0)
    (Utilities|FlowControl|Delay 0.6)
    (Actor|DestroyActor)))

(fn ConstructionScript)